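; BP_BaseShekelStation is a station actor that passively farms Shekel currency over time.
; A looping timer started on BeginPlay calls FarmShekel at the farm rate, adding the per-farm amount to the station's running total.
; Each farm shows a brief green debug string just above the actor with the gain, while Tick prints the current total on screen every frame.
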(event EventBeginPlay
  (Utilities|Time|SetTimerbyFunctionName 0 "FarmShekel" (Variables|Default|GetFarmRate) true))

(event Collision|EventActorBeginOverlap
  (params (OtherActor :type Actor%20Object%20Reference)))

(event EventTick
  (params (DeltaSeconds :type Float%20%28single-precision%29))
  (Development|PrintString (Utilities|String|ToString(Text) (Utilities|Text|FormatText "Shekel:{Shekel}" (Variables|Default|GetTotalShekel))) true false "(R=0.000000,G=0.660000,B=1.000000,A=1.000000)" 0.0))

(fn ConstructionScript)

(fn FarmShekel
  (Variables|Default|SetTotalShekel (+ (Variables|Default|GetShekelPerFarm) (Variables|Default|GetTotalShekel)))
  (Rendering|Debug|DrawDebugString (+ (Transformation|GetActorLocation) "-2.000000, 0,15.000000") (Utilities|String|ToString(Text) (Utilities|Text|FormatText "+{Shekel}" (Variables|Default|GetShekelPerFarm))) 0 "(R=0.224021,G=1.000000,B=0.034841,A=1.000000)" 0.5))