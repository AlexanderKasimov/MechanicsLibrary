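; Player-controlled 2D turret that aims its Paper2D sprite at the mouse cursor and fires a hitscan laser on left click.
; Each tick, a cursor Visibility trace stores the target point and rotates the sprite toward it.
; A click draws a debug-line beam from the Muzzle socket with a colored impact particle, then sends DamageMessage to any IDamageble actor under the cursor.
; Several disconnected debug and experimental rotation chains never run.
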(event EventBeginPlay
  (Input|EnableInput (Game|GetPlayerController 0)))

(event EventTick
  (params (DeltaSeconds :type Float%20%28single-precision%29))
  (bind _returnvalue (Game|GetPlayerController 0))
  (bind (_hitresult _returnvalue_2) (Game|Player|GetHitResultUnderCursorbyChannel _returnvalue "TraceTypeQuery1" true))
  (bind _location (Collision|BreakHitResult _hitresult))
  (bind _returnvalue_3 (+ _location "0,1.000000,0.000000"))
  (if _returnvalue_2
    (Variables|Default|SetMouseLocation _returnvalue_3)
    (Transformation|SetWorldRotation (Variables|Default|GetPaperSprite1) (Math|Conversions|RotationFromXVector (- _returnvalue_3 (Transformation|GetWorldLocation (Variables|Default|GetPaperSprite1)))) false false)))

(event Input|MouseEvents|LeftMouseButton
  (params (Key :type Key%20Structure))
  (bind _returnvalue (Game|GetPlayerController 0))
  (bind (_hitresult _returnvalue_2) (Game|Player|GetHitResultUnderCursorbyChannel _returnvalue "TraceTypeQuery1" true))
  (bind _hitactor (Collision|BreakHitResult _hitresult))
  (:Pressed
    (Utilities|FlowControl|Sequence
      (:then_0
        (Rendering|Debug|DrawDebugLine (Transformation|GetSocketLocation (Variables|Default|GetPaperSprite1) "Muzzle") (Variables|Default|GetMouseLocation) (Variables|Default|GetLazerColor) 0.4 1.0)
        (bind _returnvalue_3 (Effects|SpawnEmitteratLocation "/Game/Particles/P_collision2.P_collision2" (Variables|Default|GetMouseLocation)))
        (Effects|Components|ParticleSystem|SetColorParameter _returnvalue_3 "Color" (Variables|Default|GetLazerColor)))
      (:then_1
        (if _returnvalue_2
          (if (Utilities|DoesObjectImplementInterface _hitactor "/Game/Saliens/BP/IDamageble.IDamageble_C")
            (Class|IDamageble|Damage(Message) _hitactor (Variables|Default|GetDamage))))))))

(fn ConstructionScript)