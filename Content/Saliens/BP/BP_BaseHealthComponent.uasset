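; BP_BaseHealthComponent is a base health component that tracks hit points for the actor that owns it.
; It sets current HP to max HP on BeginPlay, and its Damage event subtracts the incoming amount.
; When HP drops to zero or below, it calls HandleDeathMessage on the owner, leaving the death response to that actor.
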(event EventBeginPlay
  (Variables|Default|SetCurHP (Variables|Default|GetMaxHP)))

(event EventTick
  (params (DeltaSeconds :type Float%20%28single-precision%29)))

(event EventDamage
  (params (Damage :type Float%20%28single-precision%29))
  (Variables|Default|SetCurHP (- (Variables|Default|GetCurHP) Damage))
  (if (CallFunction|CheckIsDead)
    (Class|IDamageble|HandleDeath(Message) (Components|GetOwner))))

(fn CheckIsDead
  (return (<= (Variables|Default|GetCurHP) 0.0)))