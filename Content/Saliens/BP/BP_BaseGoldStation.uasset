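; BP_BaseGoldStation is a gold-producing station that passively adds to its own gold total on a looping timer.
; Each farm tick shows a floating debug "+gold" label above the actor, while Tick prints the running total on screen.
; Its non-looping flipbook starts stopped and replays at random intervals, re-armed by a periodic check that skips scheduling while a play timer is active.
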(event OnFinishedPlaying(PaperFlipbook)
  (Development|PrintString "Hello"))

(event EventBeginPlay
  (Utilities|Time|SetTimerbyFunctionName 0 "FarmGold" (Variables|Default|GetFarmRate) true)
  (Components|Timeline|SetLooping (Variables|Default|GetPaperFlipbook) false)
  (Audio|Components|Audio|Stop (Variables|Default|GetPaperFlipbook))
  (Class|PaperFlipbookComponent|SetPlaybackPositioninFrames (Variables|Default|GetPaperFlipbook) 0 false)
  (CallFunction|SetPlayAnimationTimer)
  (Utilities|Time|SetTimerbyFunctionName 0 "SetPlayAnimationTimer" 7.0 true))

(event Collision|EventActorBeginOverlap
  (params (OtherActor :type Actor%20Object%20Reference)))

(event EventTick
  (params (DeltaSeconds :type Float%20%28single-precision%29))
  (Development|PrintString (Utilities|String|ToString(Text) (Utilities|Text|FormatText "Gold:{Gold}" (Variables|Default|GetTotalGold))) true false "(R=0.000000,G=0.660000,B=1.000000,A=1.000000)" 0.0))

(fn ConstructionScript)

(fn FarmGold
  (Variables|Default|SetTotalGold (+ (Variables|Default|GetGoldPerFarm) (Variables|Default|GetTotalGold)))
  (Rendering|Debug|DrawDebugString (+ (Transformation|GetActorLocation) "-2.000000, 0,15.000000") (Utilities|String|ToString(Text) (Utilities|Text|FormatText "+{Gold}" (Variables|Default|GetGoldPerFarm))) 0 "(R=0.224021,G=1.000000,B=0.034841,A=1.000000)" 0.5))

(fn PlayAnimation
  (Components|Timeline|PlayfromStart (Variables|Default|GetPaperFlipbook)))

(fn SetPlayAnimationTimer
  (if (not (Utilities|Time|IsTimerActivebyHandle (Variables|Default|GetPlayAnimationTimerHandle)))
    (bind _returnvalue (Utilities|Time|SetTimerbyFunctionName 0 "PlayAnimation" (Math|Random|RandomFloatinRange 5.0 15.0)))
    (Variables|Default|SetPlayAnimationTimerHandle _returnvalue)))