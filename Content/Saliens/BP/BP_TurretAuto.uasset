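; Automatic turret that locks onto the nearest actor tagged "Enemy" and shoots it with a laser.
; Activated on BeginPlay, it runs two looping timers: a once-per-second scan of all tagged actors for the closest, and a fire timer paced by FireRate.
; Tick rotates the barrel sprite toward the target.
; Each shot plays laser and explosion effects at the target's location, then deals damage directly, without a trace or projectile in this graph.
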(event Custom|Activate
  (bind _returnvalue (Utilities|Time|SetTimerbyFunctionName 0 "SetTarget" 1.0 true))
  (Variables|Default|SetSetTargetTimerHandle _returnvalue)
  (Utilities|Time|SetTimerbyFunctionName 0 "Fire" (/ 1.0 (Variables|Default|GetFireRate)) true))

(event EventBeginPlay
  (Variables|Default|SetTarget 0)
  (CallFunction|Activate))

(event EventTick
  (params (DeltaSeconds :type Float%20%28single-precision%29))
  (if (CallFunction|HasTarget)
    (Transformation|SetWorldRotation (Variables|Default|GetBarrelSprite) (Math|Conversions|RotationFromXVector (- (Transformation|GetActorLocation (Variables|Default|GetTarget)) (Transformation|GetWorldLocation (Variables|Default|GetBarrelSprite)))) false false)))

(fn ConstructionScript
  (|CallParentFunction))

(fn GetTarget
  (LocalVariables|SetBestTarget 0)
  (LocalVariables|SetClosestDistance 1e+08)
  (bind _outactors (Actor|GetAllActorswithTag "Enemy"))
  (for _array_element _outactors
    (bind _output_get (LocalVariables|SetCurActor _array_element))
    (if (< (Transformation|GetDistanceTo _output_get self) (LocalVariables|GetClosestDistance))
      (LocalVariables|SetBestTarget (LocalVariables|GetCurActor))
      (LocalVariables|SetClosestDistance (Transformation|GetDistanceTo _output_get self))))
  (return (LocalVariables|GetBestTarget) (!= (LocalVariables|GetBestTarget) 0)))

(fn HasTarget
  (Utilities|IsValid (Variables|Default|GetTarget)
    (:Is%20Valid
      (return (!= (Variables|Default|GetTarget) 0)))
    (:Is%20Not%20Valid
      (return false))))

(fn SetTarget
  (bind (_target _result) (CallFunction|GetTarget))
  (if _result
    (Variables|Default|SetTarget _target)))

(fn Fire
  (if (CallFunction|HasTarget)
    (CallFunction|PlayFireEffects (Transformation|GetActorLocation (Variables|Default|GetTarget)) (Variables|Default|GetLazerColor) (Variables|Default|GetExplosionScale))
    (CallFunction|DealDamage (Variables|Default|GetTarget))))