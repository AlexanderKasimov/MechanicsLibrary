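; Base game mode for Saliens that spawns waves of enemies throughout play.
; BeginPlay spawns a wave at once and starts a looping timer, stored as a handle, that calls SpawnWave every few seconds.
; Each wave spawns a small random number of BP_BaseEnemy actors at random X and Z positions within a narrow band on a fixed Y plane.
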(event EventBeginPlay
  (CallFunction|SpawnWave)
  (bind _returnvalue (Utilities|Time|SetTimerbyFunctionName 0 "SpawnWave" 3.0 true))
  (Variables|Default|SetSpawnWaveTimerHandle _returnvalue))

(event EventTick
  (params (DeltaSeconds :type Float%20%28single-precision%29)))

(fn ConstructionScript)

(fn SpawnWave
  (bind _output_get (LocalVariables|SetEnemiesCount (Math|Random|RandomInteger 4)))
  (for _index (range 0 _output_get)
    (Game|SpawnActorfromClass "/Game/Saliens/BP/BP_BaseEnemy.BP_BaseEnemy_C" (Math|Transform|MakeTransform (Math|Vector|MakeVector (Math|Random|RandomFloatinRange 125.0 1.4e+02) 2.0 (Math|Random|RandomFloatinRange -1.2e+02 1.2e+02))) "Undefined" 0 "(R=1.000000,G=0.000000,B=0.000000,A=1.000000)" 0)))