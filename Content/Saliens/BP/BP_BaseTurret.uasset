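; Base turret Blueprint with a barrel sprite, providing shared helpers for firing effects and dealing damage.
; PlayFireEffects draws a timed debug line as the laser from the barrel's Muzzle socket to the hit location, then spawns a scaled, colored impact emitter there.
; DealDamage looks up the hit actor's BP_BaseHealthComponent and passes the damage to it.
; The event graph holds only disconnected, deprecated cursor-aiming and debug-print experiments.
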(fn ConstructionScript)

(fn PlayFireEffects
  (params (HitLocation :type Vector) (LazerColor :type Linear%20Color%20Structure) (ExplosionScale :type Float%20%28single-precision%29))
  (LocalVariables|SetLocalHitLocation HitLocation)
  (LocalVariables|SetLocalColor LazerColor)
  (LocalVariables|SetLocalExplosionScale ExplosionScale)
  (Rendering|Debug|DrawDebugLine (Transformation|GetSocketLocation (Variables|Default|GetBarrelSprite) "Muzzle") (LocalVariables|GetLocalHitLocation) (LocalVariables|GetLocalColor) 0.4 1.0)
  (bind _returnvalue (Effects|SpawnEmitteratLocation "/Game/Particles/P_collision2.P_collision2" (LocalVariables|GetLocalHitLocation) "0, 0, 0" (Math|Vector|MakeVector (LocalVariables|GetLocalExplosionScale) (LocalVariables|GetLocalExplosionScale) (LocalVariables|GetLocalExplosionScale))))
  (Effects|Components|ParticleSystem|SetColorParameter _returnvalue "Color" (LocalVariables|GetLocalColor)))

(fn DealDamage
  (params (HittedActor :type Actor%20Object%20Reference))
  (bind _returnvalue (Actor|GetComponentbyClass HittedActor "/Game/Saliens/BP/BP_BaseHealthComponent.BP_BaseHealthComponent_C"))
  (Utilities|IsValid _returnvalue
    (:Is%20Valid
      (Class|IDamageble|Damage(Message) _returnvalue (Variables|Default|GetDamage)))))