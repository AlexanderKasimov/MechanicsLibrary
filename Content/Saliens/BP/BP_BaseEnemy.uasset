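; BP_BaseEnemy is a base enemy in Saliens that moves in a straight step each tick and damages what it rams.
; It tints its Paper2D sprite on BeginPlay, then uses a swept SetActorLocation for both movement and collision detection.
; When the move fails against an actor with BP_BaseHealthComponent, it deals damage, spawns a tinted explosion and destroys itself.
; HandleDeath destroys it without the effect.
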(event EventBeginPlay
  (Sprite|SetSpriteColor (Variables|Default|GetPaperSprite) (Variables|Default|GetEnemyColor)))

(event EventHandleDeath
  (Actor|DestroyActor))

(event EventTick
  (params (DeltaSeconds :type Float%20%28single-precision%29))
  (bind (_sweephitresult _returnvalue) (Transformation|SetActorLocation (+ (Transformation|GetActorLocation) (* (Variables|Default|GetMoveDirection) (Variables|Default|GetMoveSpeed))) true false))
  (if (not _returnvalue)
    (Utilities|IsValid (Actor|GetComponentbyClass (.HitActor (Collision|BreakHitResult _sweephitresult)) "/Game/Saliens/BP/BP_BaseHealthComponent.BP_BaseHealthComponent_C")
      (:Is%20Valid
        (Class|IDamageble|Damage(Message) (Actor|GetComponentbyClass (.HitActor (Collision|BreakHitResult _sweephitresult)) "/Game/Saliens/BP/BP_BaseHealthComponent.BP_BaseHealthComponent_C") (Variables|Default|GetAttackDamage))
        (bind _returnvalue_2 (Effects|SpawnEmitteratLocation "/Game/Particles/P_collision2.P_collision2" (Transformation|GetActorLocation) "0, 0, 0" "0.500000,0.500000,0.500000"))
        (Effects|Components|ParticleSystem|SetColorParameter _returnvalue_2 "Color" (Variables|Default|GetExplosionColor))
        (Actor|DestroyActor)))))

(fn ConstructionScript)