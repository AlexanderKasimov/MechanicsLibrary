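; Player-controlled turret in Saliens that aims its barrel at the mouse cursor and fires a laser on left click.
; Each tick it traces under the cursor, stores the hit point nudged along Y and rotates the barrel sprite toward it.
; A click plays fire effects at the stored point, then re-traces under the cursor and passes any hit actor to DealDamage.
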(event EventBeginPlay
  (Input|EnableInput (Game|GetPlayerController 0)))

(event Collision|EventActorBeginOverlap
  (params (OtherActor :type Actor%20Object%20Reference)))

(event EventTick
  (params (DeltaSeconds :type Float%20%28single-precision%29))
  (bind _returnvalue (Game|GetPlayerController 0))
  (bind (_hitresult _returnvalue_2) (Game|Player|GetHitResultUnderCursorbyChannel _returnvalue "TraceTypeQuery1" true))
  (bind _location (Collision|BreakHitResult _hitresult))
  (bind _returnvalue_3 (+ _location "0,1.000000,0.000000"))
  (if _returnvalue_2
    (Variables|Default|SetMouseLocation _returnvalue_3)
    (Transformation|SetWorldRotation (Variables|Default|GetBarrelSprite) (Math|Conversions|RotationFromXVector (- _returnvalue_3 (Transformation|GetWorldLocation (Variables|Default|GetBarrelSprite)))) false false)))

(event Input|MouseEvents|LeftMouseButton
  (params (Key :type Key%20Structure))
  (bind _returnvalue (Game|GetPlayerController 0))
  (bind (_hitresult _returnvalue_2) (Game|Player|GetHitResultUnderCursorbyChannel _returnvalue "TraceTypeQuery1" true))
  (:Pressed
    (Utilities|FlowControl|Sequence
      (:then_0
        (CallFunction|PlayFireEffects (Variables|Default|GetMouseLocation) (Variables|Default|GetLazerColor) (Variables|Default|GetExplosionScale)))
      (:then_1
        (if _returnvalue_2
          (CallFunction|DealDamage (.HitActor (Collision|BreakHitResult _hitresult))))))))

(fn ConstructionScript
  (|CallParentFunction))