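; Player character for a Titan Souls-style training project, a Paper2D sprite rotated in the construction script, with movement and a timed dodge.
; Tick moves it by swept SetActorLocation along the normalized input direction, using per-frame speeds without delta-time scaling.
; Dodge locks that direction at dodge speed, reflecting it off the first blocking surface hit.
; FinishDodge ends the dodge on a timer and restores the saved direction.
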(event EventBeginPlay
  (Variables|Default|SetCurMoveDirection "1.000000, 0, 0"))

(event Collision|EventActorBeginOverlap
  (params (OtherActor :type Actor%20Object%20Reference)))

(event EventTick
  (params (DeltaSeconds :type Float%20%28single-precision%29))
  (if (not (Variables|Default|GetisDodging))
    (if (or (> (Math|Float|Absolute(Float) (Input|AxisValues|GetMoveUp)) 0.0) (> (Math|Float|Absolute(Float) (Input|AxisValues|GetMoveRight)) 0.0))
      (Variables|Default|SetCurMoveDirection (Math|Vector|Normalize (Math|Vector|MakeVector (Input|AxisValues|GetMoveUp) (Input|AxisValues|GetMoveRight) 0.0)))
      (Transformation|SetActorLocation (+ (Transformation|GetActorLocation) (* (Variables|Default|GetCurMoveDirection) (Variables|Default|GetMoveSpeed))) true false)
      (else
        (Variables|Default|SetOldMoveDirection (Variables|Default|GetCurMoveDirection))))
    (else
      (bind (_sweephitresult _returnvalue) (Transformation|SetActorLocation (+ (Transformation|GetActorLocation) (* (Variables|Default|GetCurMoveDirection) (Variables|Default|GetDodgeSpeed))) true false))
      (if (not _returnvalue)
        (if (not (Variables|Default|GetisCollided))
          (Utilities|FlowControl|Sequence
            (:then_0
              (Variables|Default|SetisCollided true)
              (Variables|Default|SetOldMoveDirection (Variables|Default|GetCurMoveDirection)))
            (:then_1
              (Variables|Default|SetCurMoveDirection (Math|Vector|GetReflectionVector (Variables|Default|GetCurMoveDirection) (.Normal (Collision|BreakHitResult _sweephitresult)))))))))))

(event Input|ActionEvents|InputActionDodge
  (params (Key :type Key%20Structure))
  (:Pressed
    (if (not (Variables|Default|GetisDodging))
      (Variables|Default|SetisDodging true)
      (Utilities|Time|SetTimerbyFunctionName 0 "FinishDodge" (Variables|Default|GetDodgeTime)))))

(fn ConstructionScript
  (Transformation|SetRelativeRotation (Variables|Default|GetPaperSprite) "0.000000, 0,90.000000" false false))

(fn FinishDodge
  (Variables|Default|SetisDodging false)
  (Variables|Default|SetCurMoveDirection (Variables|Default|GetOldMoveDirection))
  (Variables|Default|SetisCollided false))